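; BP_HiddenLevelDoor is an interactable door that leads to a hidden level once no collectibles remain.
; A Box overlap with TPC_Main enables Interact input on the actor, and leaving disables it.
; Interact checks CollectibleLeft on ThirdPersonGameMode, then plays a timeline that yaws StaticMesh2.
; The timeline's Update also feeds a Delay that opens HiddenLevel shortly after the swing starts.
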(event `InputAction|Interact`
  (params (Key :type "Key Structure"))
  (:`Pressed`
    (bind _asthird_person_game_mode (cast `/Game/ThirdPersonBP/Blueprints/ThirdPersonGameMode` (`GameplayStatics.GetGameMode`)))
    (if (== (`/Game/ThirdPersonBP/Blueprints/ThirdPersonGameMode.CollectibleLeft` _asthird_person_game_mode) 0)
      (bind (_direction _newtrack_0) (`Timeline|Open/Close Door` :!via `PlayFromStart`)
        (:`Update`
          (`SceneComponent.K2_SetRelativeRotation` (`self.StaticMesh2`) (`KismetMathLibrary.MakeRotator` 0.0 0.0 _newtrack_0) false false)
          (`KismetSystemLibrary.Delay` 2.0)
          (`GameplayStatics.OpenLevelBySoftObjectPtr` "/Game/1GameFiles/Levels/HiddenLevel.HiddenLevel"))))))

(event `self.Box.OnComponentBeginOverlap`
  (params (OverlappedComponent :type "PrimitiveComponent Object Reference") (OtherActor :type "Actor Object Reference") (OtherComp :type "PrimitiveComponent Object Reference") (OtherBodyIndex :type Integer) (bFromSweep :type Boolean) (SweepResult :type "HitResult Structure (by ref)"))
  (cast `/Game/1GameFiles/TPC_Main` OtherActor)
  (`self.EnableInput` (`GameplayStatics.GetPlayerController` 0)))

(event `self.Box.OnComponentEndOverlap`
  (params (OverlappedComponent :type "PrimitiveComponent Object Reference") (OtherActor :type "Actor Object Reference") (OtherComp :type "PrimitiveComponent Object Reference") (OtherBodyIndex :type Integer))
  (cast `/Game/1GameFiles/TPC_Main` OtherActor)
  (`self.DisableInput` (`GameplayStatics.GetPlayerController` 0)))

(fn `UserConstructionScript`)